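; Player flying pawn that steers with axis input and mouse look through a floating pawn movement component, with a held boost multiplying max speed.
; Left click fires a debug-drawn sphere trace along the forward vector to find a CancerCell.
; On a hit, it tells FlyingGameMode to begin the fight animation at the impact point, then hides both itself and the cell.
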(event EventBeginPlay
  (Variables|Default|SetDefaultMaxSpeed (Class|MovementComponent|GetMaxSpeed (Variables|Default|GetFloatingPawnMovement))))

(event Input|ActionEvents|InputActionBoost
  (params (Key :type Key%20Structure :default "None"))
  (bind _floatingpawnmovement (Variables|Default|GetFloatingPawnMovement))
  (:Pressed
    (Variables|/Script/Engine.FloatingPawnMovement|SetMaxSpeed _floatingpawnmovement (* (Variables|Default|GetDefaultMaxSpeed) (Variables|Default|GetBoostMultiplier))))
  (:Released
    (Variables|/Script/Engine.FloatingPawnMovement|SetMaxSpeed _floatingpawnmovement (Variables|Default|GetDefaultMaxSpeed))))

(event Input|AxisEvents|InputAxisForward
  (params (AxisValue :type Float%20%28single-precision%29))
  (Class|PawnMovementComponent|AddInputVector (Variables|Default|GetFloatingPawnMovement) (* (* (Transformation|GetActorForwardVector) AxisValue) (Class|MovementComponent|GetMaxSpeed (Variables|Default|GetFloatingPawnMovement))) false))

(event Input|AxisEvents|InputAxisRight
  (params (AxisValue :type Float%20%28single-precision%29))
  (Class|PawnMovementComponent|AddInputVector (Variables|Default|GetFloatingPawnMovement) (* (* (Transformation|GetActorRightVector) AxisValue) (Class|MovementComponent|GetMaxSpeed (Variables|Default|GetFloatingPawnMovement))) false))

(event Input|AxisEvents|InputAxisMouse_X_Input
  (params (AxisValue :type Float%20%28single-precision%29))
  (Transformation|AddActorLocalRotation (Math|Rotator|MakeRotator 0.0 0.0 (* AxisValue (Variables|Default|GetLookSpeed))) false false))

(event Input|AxisEvents|InputAxisMouse_Y_Input
  (params (AxisValue :type Float%20%28single-precision%29))
  (Transformation|AddActorLocalRotation (Math|Rotator|MakeRotator 0.0 (* AxisValue (Variables|Default|GetLookSpeed)) 0.0) false false))

(event Input|MouseEvents|LeftMouseButton
  (params (Key :type Key%20Structure :default "None"))
  (bind _returnvalue (Transformation|GetActorLocation))
  (:Pressed
    (bind (_outhit _returnvalue_2) (Collision|SphereTraceByChannel _returnvalue (+ _returnvalue (* (Transformation|GetActorForwardVector) (Variables|Default|GetAttackDistance))) 1.5e+02 "TraceTypeQuery1" false 0 "ForDuration" true "(R=1.000000,G=0.000000,B=0.000000,A=1.000000)" "(R=0.000000,G=1.000000,B=0.000000,A=1.000000)" 0.5))
    (if _returnvalue_2
      (bind _ascancer_cell (Utilities|Casting|CastToCancerCell (.HitActor (Collision|BreakHitResult _outhit))))
      (Utilities|FlowControl|Sequence
        (:then_0
          (bind _asflying_game_mode (Utilities|Casting|CastToFlyingGameMode (Game|GetGameMode)))
          (Default|BeginFightAnimation _asflying_game_mode (Math|Transform|MakeTransform (.Location (Collision|BreakHitResult _outhit)))))
        (:then_1
          (CallFunction|Hide true))
        (:then_2
          (Default|Hide _ascancer_cell true))))))

(fn ConstructionScript)

(fn Hide
  (params (Hide :type Boolean))
  (Rendering|SetActorHiddenInGame Hide))