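; Cancer cell enemy that takes damage from BP_Player and, for one Type variant, ambushes the player on overlap.
; If the player is not attacking, it stuns and halts them, then a Timeline pulls the cell in and adjusts the camera before it emits smoke and activates the player's antibody.
; Hits spawn particles at the attach point; death swaps material, dissolves and calls ReturnFromAttack on the player.
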(event OnComponentBeginOverlap(Sphere1)
  (params (OverlappedComponent :type Primitive%20Component%20Object%20Reference) (OtherActor :type Actor%20Object%20Reference) (OtherComp :type Primitive%20Component%20Object%20Reference) (OtherBodyIndex :type Integer) (bFromSweep :type Boolean) (SweepResult :type Hit%20Result%20Structure%20%28by%20ref%29))
  (bind _asbp_player (Utilities|Casting|CastToBP_Player OtherActor))
  (if (Utilities|Enum|Equal(Enum) (Variables|Default|GetType) "NewEnumerator1")
    (Variables|Default|SetPlayerRef _asbp_player)
    (if (not (Variables|/Game/Core/Player/BP_Player.BP_Player_C|GetbIsAttacking? (Variables|Default|GetPlayerRef)))
      (Variables|/Game/Core/Player/BP_Player.BP_Player_C|SetbIsStunned? (Variables|Default|GetPlayerRef) true)
      (Variables|/Script/Engine.FloatingPawnMovement|SetDeceleration (Variables|/Game/Core/Player/BP_Player.BP_Player_C|GetFloatingPawnMovement _asbp_player) 8e+04)
      (Variables|/Script/Engine.FloatingPawnMovement|SetMaxSpeed (Variables|/Game/Core/Player/BP_Player.BP_Player_C|GetFloatingPawnMovement _asbp_player) 0.0)
      (bind _lerp (Timeline|Timeline_0 PlayFromStart)
        (:Update
          (Transformation|SetActorLocation (Math|Vector|Lerp(Vector) (Transformation|GetActorLocation) (+ (Transformation|GetActorLocation (Variables|Default|GetPlayerRef)) (* (Transformation|GetActorForwardVector) 75.0)) _lerp) false false)
          (Default|SetCameraDistance (Variables|Default|GetPlayerRef) _lerp))
        (:Finished
          (CallFunction|Attacking))))))

(event Custom|GetAttachLocation
  (params (AttachPoint :type Vector))
  (Variables|Default|SetAttachLocation AttachPoint))

(event Custom|Attacking
  (bind _returnvalue (Transformation|GetActorTransform))
  (bind _playerref (Variables|Default|GetPlayerRef))
  (bind (_location _rotation _scale) (Math|Transform|BreakTransform _returnvalue))
  (bind _returnvalue_2 (Niagara|SpawnSystematLocation "/Game/Particle/NE_Smoke_System.NE_Smoke_System" _location "0, 0, 0" _scale))
  (Variables|Default|SetCancerSmoke _returnvalue_2)
  (Variables|/Game/Core/Player/BP_Player.BP_Player_C|SetActiveTarget _playerref self)
  (Default|ActivateAntibody _playerref))

(event Custom|Destroy
  (Components|Activation|SetActive (Variables|Default|GetCancerSmoke) false true))

(event Game|Damage|EventAnyDamage
  (params (Damage :type Float%20%28single-precision%29) (DamageType :type Damage%20Type%20Object%20Reference) (InstigatedBy :type Controller%20Object%20Reference) (DamageCauser :type Actor%20Object%20Reference))
  (bind _returnvalue (Transformation|GetActorTransform))
  (bind _attachlocation (Variables|Default|GetAttachLocation))
  (bind (_location _rotation _scale) (Math|Transform|BreakTransform _returnvalue))
  (bind _asbp_player (Utilities|Casting|CastToBP_Player DamageCauser))
  (Variables|Default|SetPlayerRef _asbp_player)
  (Niagara|SpawnSystematLocation "/Game/Particle/NewNiagaraEmitter_System.NewNiagaraEmitter_System" (+ (Transformation|GetActorLocation) (* _attachlocation -5e+01)) (Math|Conversions|RotationFromXVector _attachlocation))
  (Variables|Default|SetHealth (- (Variables|Default|GetHealth) Damage))
  (if (<= (Variables|Default|GetHealth) 0.0)
    (Rendering|Material|SetMaterial (Variables|Default|GetCancer%20Cell) 0 (Variables|Default|GetM_DeathC))
    (Niagara|SpawnSystematLocation "/Game/Particle/NE_Dissolving_System.NE_Dissolving_System" _location _rotation _scale)
    (Default|ReturnfromAttack (Variables|Default|GetPlayerRef))
    (Actor|DestroyActor)))

(event EventBeginPlay
  (bind _returnvalue (Rendering|Material|CreateDynamicMaterialInstance (Variables|Default|GetCancer%20Cell) 0 "/Game/Assets/CancerCell/Death/Fast/CancerCell_Death_Mat_Inst.CancerCell_Death_Mat_Inst" "None" :!class /Script/Engine.PrimitiveComponent))
  (Variables|Default|SetM_DeathC _returnvalue))

(fn ConstructionScript)