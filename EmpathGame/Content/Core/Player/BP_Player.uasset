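; Player pawn that flies with floating movement and hunts cancer cells.
; Attack input sphere-traces along the view for a BP_CancerCell, then a timeline dashes to it and pulls the spring arm into fight distance.
; Further presses deal damage with effects and camera shake, or build antibodies when stunned until the cell is destroyed.
; ReturnFromAttack reverses the timeline to restore normal movement; super mode and pitch look are unwired.
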(event Custom|AttackInitiation
  (params (SuperJump :type Vector))
  (Variables|Default|SetLastVelo (Transformation|GetVelocity))
  (Variables|Default|SetbIsAttacking? true)
  (Variables|Default|SetbResetState? false)
  (bind _lerp (Timeline|Timeline_0 PlayFromStart)
    (:Update
      (CallFunction|SetCameraDistance _lerp)
      (if (not (Variables|Default|GetbResetState?))
        (Utilities|SetPlayerAttackDash _lerp SuperJump)
        (Variables|/Script/Engine.FloatingPawnMovement|SetMaxSpeed (Variables|Default|GetFloatingPawnMovement) 0.0)))
    (:Finished
      (Utilities|OnStateChanged))))

(event Custom|ReturnFromAttack
  (Variables|Default|SetbResetState? true)
  (bind _lerp (Timeline|Timeline_0 ReverseFromEnd)
    (:Update
      (CallFunction|SetCameraDistance _lerp)
      (if (not (Variables|Default|GetbResetState?))
        (Utilities|SetPlayerAttackDash _lerp (stale Custom|AttackInitiation SuperJump))
        (Variables|/Script/Engine.FloatingPawnMovement|SetMaxSpeed (Variables|Default|GetFloatingPawnMovement) 0.0)))
    (:Finished
      (Utilities|OnStateChanged))))

(event EventBeginPlay)

(event Input|ActionEvents|InputActionAttack
  (params (Key :type Key%20Structure :default "None"))
  (:Pressed
    (if (Variables|Default|GetbIsStunned?)
      (CallFunction|UseAntibodies)
      (elif (Variables|Default|GetbIsAttacking?)
        (CallFunction|Attack)
        (elif (not (Variables|Default|GetbResetState?))
          (bind _location (Utilities|FindTarget)
            (:TargetFound
              (CallFunction|AttackInitiation _location))))))))

(fn ConstructionScript)

(fn ActivateSuperWeaponized
  (Variables|/Script/Engine.FloatingPawnMovement|SetMaxSpeed (Variables|Default|GetFloatingPawnMovement) (Variables|Default|GetSuperSpeed))
  (Variables|Default|SetAttackDistance 5e+03))

(fn TraceSettings
  (bind _returnvalue (Transformation|GetActorLocation))
  (return _returnvalue (+ _returnvalue (* (Math|Vector|GetForwardVector (Pawn|GetControlRotation :!class /Script/Engine.Pawn)) (Variables|Default|GetAttackDistance)))))

(fn Attack
  (bind _returnvalue (Transformation|GetActorTransform))
  (bind (_location _rotation _scale) (Math|Transform|BreakTransform _returnvalue))
  (Effects|SpawnEmitteratLocation "/Game/StarterContent/Particles/P_EffectBoost.P_EffectBoost" _location _rotation _scale)
  (Class|PlayerCameraManager|PlayCameraShake (Game|GetPlayerCameraManager 0) "/Game/Assets/BP/BP_CameraShake.BP_CameraShake_C" 1.0 "CameraLocal" "0, 0, 0")
  (Game|Damage|ApplyDamage (Variables|Default|GetActiveTarget) 25.0 0 self))

(fn UseAntibodies
  (bind _output_get (Variables|Default|SetAntibodyLevel (+ (Variables|Default|GetAntibodyLevel) 0.1)))
  (if (>= _output_get 1.0)
    (Variables|Default|SetbIsStunned? false)
    (Variables|Default|SetbIsAttacking? true)
    (Default|Destroy (Variables|Default|GetActiveTarget))
    (Variables|Default|SetAntibodyLevel 0.0)))

(fn SetCameraDistance
  (params (Alpha :type Float%20%28single-precision%29))
  (Variables|/Script/Engine.SpringArmComponent|SetTargetArmLength (Variables|Default|GetSpringArm) (Math|Float|Lerp (Variables|Default|GetMovingSpringArmLength) (Variables|Default|GetFightSpringArmLength) Alpha)))

(event Input|AxisEvents|InputAxisForward
  (params (AxisValue :type Float%20%28single-precision%29))
  (Pawn|Input|AddMovementInput (Math|Vector|GetForwardVector (Pawn|GetControlRotation :!class /Script/Engine.Pawn)) AxisValue false))

(event Input|AxisEvents|InputAxisRight
  (params (AxisValue :type Float%20%28single-precision%29))
  (Pawn|Input|AddMovementInput (Math|Vector|GetRightVector (Pawn|GetControlRotation :!class /Script/Engine.Pawn)) AxisValue false))

(event Input|AxisEvents|InputAxisMoveUp
  (params (AxisValue :type Float%20%28single-precision%29))
  (Pawn|Input|AddMovementInput (Transformation|GetActorUpVector) (/ AxisValue 2.0) false))

(event Input|AxisEvents|InputAxisMouse_X_Input
  (params (AxisValue :type Float%20%28single-precision%29))
  (Pawn|Input|AddControllerYawInput AxisValue))

(event Input|AxisEvents|InputAxisMouse_Y_Input
  (params (AxisValue :type Float%20%28single-precision%29))
  ;[1 1 1] Do we need this??????
)