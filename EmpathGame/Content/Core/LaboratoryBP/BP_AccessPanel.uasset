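; BP_AccessPanel is a laboratory access panel that can unlock the door it controls.
; Its Box overlap registers the panel on BP_LabCharacter and shows a "Press E to Access" overlay; end overlap clears the reference but leaves that widget in place.
; Access passes the panel to EnterName on its WB_Panel widget.
; OpenDoor clears IsLocked on ControlledDoor, with no caller in this graph.
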(event OnComponentBeginOverlap(Box)
  (params (OverlappedComponent :type Primitive%20Component%20Object%20Reference) (OtherActor :type Actor%20Object%20Reference) (OtherComp :type Primitive%20Component%20Object%20Reference) (OtherBodyIndex :type Integer) (bFromSweep :type Boolean) (SweepResult :type Hit%20Result%20Structure%20%28by%20ref%29))
  (bind _asbp_lab_character (Utilities|Casting|CastToBP_LabCharacter OtherActor))
  (Variables|/Game/Core/LaboratoryBP/BP_LabCharacter.BP_LabCharacter_C|SetAccessPanel _asbp_lab_character self)
  (Variables|/Game/Core/LaboratoryBP/BP_LabCharacter.BP_LabCharacter_C|SetbIsOverlappingPanel _asbp_lab_character true)
  (bind _returnvalue (UserInterface|CreateWidget "/Game/Core/LaboratoryBP/Overlay.Overlay_C" 0 "Press E to Access"))
  (UserInterface|Viewport|AddtoViewport _returnvalue 0))

(event OnComponentEndOverlap(Box)
  (params (OverlappedComponent :type Primitive%20Component%20Object%20Reference) (OtherActor :type Actor%20Object%20Reference) (OtherComp :type Primitive%20Component%20Object%20Reference) (OtherBodyIndex :type Integer))
  (bind _asbp_lab_character (Utilities|Casting|CastToBP_LabCharacter OtherActor))
  (Variables|/Game/Core/LaboratoryBP/BP_LabCharacter.BP_LabCharacter_C|SetAccessPanel _asbp_lab_character 0)
  (Variables|/Game/Core/LaboratoryBP/BP_LabCharacter.BP_LabCharacter_C|SetbIsOverlappingPanel _asbp_lab_character false))

(event Custom|Access
  (bind _aswb_panel (Utilities|Casting|CastToWB_Panel (UserInterface|GetUserWidgetObject (Variables|Default|GetWidget))))
  (Default|EnterName _aswb_panel self))

(event Custom|OpenDoor
  (Variables|/Game/Core/LaboratoryBP/BP_Door.BP_Door_C|SetbIsLocked? (Variables|Default|GetControlledDoor) false))

(event EventBeginPlay)

(event Collision|EventActorBeginOverlap
  (params (OtherActor :type Actor%20Object%20Reference)))

(event EventTick
  (params (DeltaSeconds :type Float%20%28single-precision%29)))

(fn ConstructionScript)