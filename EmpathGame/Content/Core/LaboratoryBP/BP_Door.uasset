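; Lockable sliding double door that opens when the lab character enters its box trigger and closes when they leave.
; A timeline plays or reverses to slide both panels apart along world X, lerping from their cached start positions toward an offset from their current location.
; The overlap also sets or clears the character's DoorRef.
; When locked, it instead plays an access-required sound, gated by a DoOnce that resets after a delay on exit.
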(event OnComponentBeginOverlap(Box)
  (params (OverlappedComponent :type Primitive%20Component%20Object%20Reference) (OtherActor :type Actor%20Object%20Reference) (OtherComp :type Primitive%20Component%20Object%20Reference) (OtherBodyIndex :type Integer) (bFromSweep :type Boolean) (SweepResult :type Hit%20Result%20Structure%20%28by%20ref%29))
  (bind _asbp_lab_character (Utilities|Casting|CastToBP_LabCharacter OtherActor))
  (Variables|/Game/Core/LaboratoryBP/BP_LabCharacter.BP_LabCharacter_C|SetDoorRef _asbp_lab_character self)
  (if (Variables|Default|GetbIsLocked?)
    (Utilities|FlowControl|DoOnce false
      (:Completed
        (Audio|PlaySoundatLocation "/Game/Core/LaboratoryBP/DemoVoice/Access_required.Access_required" (Transformation|GetActorLocation) "0, 0, 0" 1.0 1.0 0.0 0 0 0)))
    (else
      (CallFunction|OpenDoors))))

(event OnComponentEndOverlap(Box)
  (params (OverlappedComponent :type Primitive%20Component%20Object%20Reference) (OtherActor :type Actor%20Object%20Reference) (OtherComp :type Primitive%20Component%20Object%20Reference) (OtherBodyIndex :type Integer))
  (bind _asbp_lab_character (Utilities|Casting|CastToBP_LabCharacter OtherActor))
  (Variables|/Game/Core/LaboratoryBP/BP_LabCharacter.BP_LabCharacter_C|SetDoorRef _asbp_lab_character 0)
  (if (Variables|Default|GetbIsLocked?)
    (Utilities|FlowControl|Delay 3.0)
    (Utilities|FlowControl|DoOnce false) ; enters at Reset
    (else
      (CallFunction|CloseDoors))))

(event Custom|OpenDoors
  (bind _newtrack_1 (Timeline|Timeline_0 Play)
    (:Update
      (Utilities|DoorSliding (Variables|Default|GetDoorRight) (Variables|Default|GetRightDoorOriginalLoc) "60.000000,0.000000,0.000000" _newtrack_1)
      (Utilities|DoorSliding (Variables|Default|GetDoorLeft) (Variables|Default|GetLeftDoorOriginalLoc) "-60.000000,0.000000,0" _newtrack_1))))

(event Custom|CloseDoors
  (bind _newtrack_1 (Timeline|Timeline_0 Reverse)
    (:Update
      (Utilities|DoorSliding (Variables|Default|GetDoorRight) (Variables|Default|GetRightDoorOriginalLoc) "60.000000,0.000000,0.000000" _newtrack_1)
      (Utilities|DoorSliding (Variables|Default|GetDoorLeft) (Variables|Default|GetLeftDoorOriginalLoc) "-60.000000,0.000000,0" _newtrack_1))))

(event EventBeginPlay
  (Variables|Default|SetLeftDoorOriginalLoc (Transformation|GetWorldLocation (Variables|Default|GetDoorLeft)))
  (Variables|Default|SetRightDoorOriginalLoc (Transformation|GetWorldLocation (Variables|Default|GetDoorRight))))

(fn ConstructionScript)