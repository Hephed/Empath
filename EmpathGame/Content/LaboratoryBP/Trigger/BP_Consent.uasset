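; BP_Consent is a laboratory trigger that shows a cutscene widget and records the player's consent.
; The first time BP_LabCharacter enters the Box, it creates a Cutscenes widget with that character as PlayerRef and adds it to the viewport.
; The first exit sets the character's HasConsent flag and plays the consent-received sound at the trigger.
; Separate DoOnce gates keep each response to a single firing.
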(event OnComponentBeginOverlap(Box)
  (params (OverlappedComponent :type Primitive%20Component%20Object%20Reference) (OtherActor :type Actor%20Object%20Reference) (OtherComp :type Primitive%20Component%20Object%20Reference) (OtherBodyIndex :type Integer) (bFromSweep :type Boolean) (SweepResult :type Hit%20Result%20Structure%20%28by%20ref%29))
  (bind _asbp_lab_character (Utilities|Casting|CastToBP_LabCharacter OtherActor))
  (Utilities|FlowControl|DoOnce false
    (:Completed
      (bind _returnvalue (UserInterface|CreateWidget "/Game/Movies/Cutscenes.Cutscenes_C" 0 _asbp_lab_character))
      (UserInterface|Viewport|AddtoViewport _returnvalue 0))))

(event OnComponentEndOverlap(Box)
  (params (OverlappedComponent :type Primitive%20Component%20Object%20Reference) (OtherActor :type Actor%20Object%20Reference) (OtherComp :type Primitive%20Component%20Object%20Reference) (OtherBodyIndex :type Integer))
  (bind _asbp_lab_character (Utilities|Casting|CastToBP_LabCharacter OtherActor))
  (Utilities|FlowControl|DoOnce false
    (:Completed
      (Variables|/Game/LaboratoryBP/BP_LabCharacter.BP_LabCharacter_C|SetbHasConsent? _asbp_lab_character true)
      (Audio|PlaySoundatLocation "/Game/LaboratoryBP/DemoVoice/consentreceived.consentreceived" (Transformation|GetActorLocation) "0, 0, 0" 1.0 1.0 0.0 0 0 0))))

(event EventBeginPlay)

(event Collision|EventActorBeginOverlap
  (params (OtherActor :type Actor%20Object%20Reference)))

(event EventTick
  (params (DeltaSeconds :type Float%20%28single-precision%29)))

(fn ConstructionScript
  (|CallParentFunction))